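; Enemy actor for the tank game that shoots by line trace, rams the player's tank and tracks its own health.
; Damage lowers health and updates a cached child-actor health bar; Tick awards the player a point and destroys the enemy when health runs out.
; ShootAt, not called within this Blueprint, applies point damage via trace, gated by a cooldown that Tick counts down.
; Colliding with a TankBP damages it and destroys the enemy without scoring.
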(event Game|Damage|EventAnyDamage
  (params (Damage :type Float%20%28single-precision%29) (DamageType :type Damage%20Type%20Object%20Reference) (InstigatedBy :type Controller%20Object%20Reference) (DamageCauser :type Actor%20Object%20Reference))
  (Variables|Default|SetHealth (- (Variables|Default|GetHealth) Damage))
  (CallFunction|UpdateHealthPercent))

(event EventBeginPlay
  (bind _output_get (Variables|Default|SetMaxHealth 1e+01))
  (Variables|Default|SetHealth _output_get)
  (Variables|Default|SetMaxShotTimer 1e+01))

(event EventActorBeginOverlap
  (params (OtherActor :type Actor%20Object%20Reference)))

(event EventTick
  (params (DeltaSeconds :type Float%20%28single-precision%29))
  (CallFunction|KillCheck)
  (CallFunction|CountdownTImers DeltaSeconds))

(event Collision|EventHit
  (params (MyComp :type Primitive%20Component%20Object%20Reference) (Other :type Actor%20Object%20Reference) (OtherComp :type Primitive%20Component%20Object%20Reference) (bSelfMoved :type Boolean) (HitLocation :type Vector :default "0, 0, 0") (HitNormal :type Vector) (NormalImpulse :type Vector) (Hit :type Hit%20Result%20Structure%20%28by%20ref%29))
  (bind _self self)
  (bind _astank_bp (Utilities|Casting|CastToTankBP Other))
  (bind _returnvalue (AI|GetAIController _self))
  (Game|Damage|ApplyPointDamage _astank_bp 1e+01 HitNormal Hit _returnvalue _self)
  (Actor|DestroyActor))

(fn ConstructionScript)

(fn Shootat
  (params (ShootAt :type Vector) (Desired :type Array%20of%20EObjectTypeQuery%20Enums) (Ignore :type Array%20of%20Actor%20Object%20References))
  (bind _self self)
  (Math|Float|CompareFloat (Variables|Default|GetShootTimer) 0.0001
    (:<
      (bind _outhit (Collision|LineTraceForObjects (Transformation|GetActorLocation) ShootAt Desired false Ignore "ForDuration"))
      (bind _returnvalue (AI|GetAIController _self))
      (Game|Damage|ApplyPointDamage (.HitActor (Collision|BreakHitResult _outhit)) 1e+01 (.ImpactNormal (Collision|BreakHitResult _outhit)) _outhit _returnvalue _self)
      (Variables|Default|SetShootTimer (Variables|Default|GetMaxShotTimer)))))

(fn KillCheck
  (Math|Float|CompareFloat (Variables|Default|GetHealth) 1.0
    (:<
      (bind _astank_bp (Utilities|Casting|CastToTankBP (Pawn|GetControlledPawn (Game|GetPlayerController 0))))
      (Default|AddScore _astank_bp 1)
      (Actor|DestroyActor))))

(fn CountdownTImers
  (params (DeltaTime :type Float%20%28single-precision%29))
  (Math|Float|CompareFloat (Variables|Default|GetShootTimer) 0.0
    (:>
      (Variables|Default|SetShootTimer (- (Variables|Default|GetShootTimer) DeltaTime)))))

(fn UpdateHealthPercent
  (Utilities|IsValid (LocalVariables|GetAiHealthActor)
    (:Is%20Valid
      _)
    (:Is%20Not%20Valid
      (bind _asenemy_ai_health (Utilities|Casting|CastToEnemyAiHealth (Variables|/Script/Engine.ChildActorComponent|GetChildActor (Variables|Default|GetHealthBar))))
      (LocalVariables|SetAiHealthActor _asenemy_ai_health)))
  (Default|UpdateHealthPercent (LocalVariables|GetAiHealthActor) (Math|Float|NormalizetoRange (Variables|Default|GetHealth) 0.0 (Variables|Default|GetMaxHealth))))